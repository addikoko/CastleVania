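; Annette NPC Blueprint that steps through a list of dialogue lines each time its Talk event fires.
; Talk increments an index, lazily creates the Annette dialogue widget, shows the line at that index and plays a coin sound cue.
; Once the index exceeds the dialogue length, it removes the widget and loops a terrified animation on the skeletal mesh.
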(event `/Game/RENJASFOLDERGTO/Annette/bpi_dialogue.talk`
  (`/Engine/EditorBlueprintResources/StandardMacros.IncrementInt` (`self.talkindex`)
    (:`  `
      (if (<= (`self.talkindex`) (`KismetArrayLibrary.Array_Length` (`self.dialogue`)))
        (`self.ui`
          (:`then`
            _)
          (:`else`
            (bind _returnvalue (`|CreateWidget` "/Game/RENJASFOLDERGTO/Annette/Annettedialoogue.Annettedialoogue_C" (`GameplayStatics.GetPlayerController` 0)))
            (bind _output_get (set `self.ui` _returnvalue))
            (`UserWidget.AddToViewport` _output_get 0)))
        (`TextBlock.SetText` (`/Game/RENJASFOLDERGTO/Annette/Annettedialoogue.TextBlock_0` (`self.ui`)) (`KismetTextLibrary.Conv_StringToText` (`|GetArrayItem` (`self.dialogue`) (`self.talkindex`))))
        (`GameplayStatics.PlaySound2D` "/Game/Interface_And_Item_Sounds/Cues/Coins_02_Cue.Coins_02_Cue" 1.0 1.0 0.0 null null)
        (else
          (`Widget.RemoveFromParent` (`self.ui`))
          (`SkeletalMeshComponent.PlayAnimation` (`self.SkeletalMesh`) "/Game/RENJASFOLDERGTO/Annette/Terrified_Anim.Terrified_Anim" true))))))

(fn `UserConstructionScript`)