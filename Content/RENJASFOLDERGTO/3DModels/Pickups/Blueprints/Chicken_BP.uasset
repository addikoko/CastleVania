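; Chicken health pickup that heals the player's third-person character on overlap, then removes itself from the world.
; It caches the player character on BeginPlay and accepts only that actor in its box overlap.
; A DoOnce gate, set to start closed if health is below zero, leads to a clamped health increase, a health update call, a collect sound and self-destruction.
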(event `self.ReceiveBeginPlay`
  (bind _asbp_third_person_character (cast `/Game/ThirdPerson/Blueprints/BP_ThirdPersonCharacter` (`GameplayStatics.GetPlayerCharacter` 0)))
  (set `self.As BP Third Person Character` _asbp_third_person_character))

(event `self.Box.OnComponentBeginOverlap`
  (params (OverlappedComponent :type "PrimitiveComponent Object Reference") (OtherActor :type "Actor Object Reference") (OtherComp :type "PrimitiveComponent Object Reference") (OtherBodyIndex :type Integer) (bFromSweep :type Boolean) (SweepResult :type "HitResult Structure (by ref)"))
  (bind _as_bp_third_person_character (`self.As BP Third Person Character`))
  (if (== OtherActor (`self.As BP Third Person Character`))
    (`/Engine/EditorBlueprintResources/StandardMacros.DoOnce` (< (`/Game/ThirdPerson/Blueprints/BP_ThirdPersonCharacter.Health` (`self.As BP Third Person Character`)) 0.0)
      (:`Completed`
        (set `/Game/ThirdPerson/Blueprints/BP_ThirdPersonCharacter.Health` (`KismetMathLibrary.FClamp` (+ (`/Game/ThirdPerson/Blueprints/BP_ThirdPersonCharacter.Health` _as_bp_third_person_character) 10.0) 0.0 (`/Game/ThirdPerson/Blueprints/BP_ThirdPersonCharacter.MaxHealth` _as_bp_third_person_character)) _as_bp_third_person_character)
        (`/Game/ThirdPerson/Blueprints/BP_ThirdPersonCharacter.UpdateHealth` _as_bp_third_person_character)
        (`GameplayStatics.PlaySoundAtLocation` "/Game/RENJASFOLDERGTO/3DModels/Pickups/sounds/Collect_Item_Sound_Effect.Collect_Item_Sound_Effect" (`self.K2_GetActorLocation`) (struct) 1.0 1.0 0.0 null null null null)
        (`self.K2_DestroyActor`)))))

(fn `UserConstructionScript`)