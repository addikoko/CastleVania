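; Trigger volume that starts a rising-flame hazard by spawning a row of BP_RisingFlame actors.
; The first Box overlap passes a DoOnce, prints a debug "Hello", then spawns the flames only if the actor is BP_ThirdPersonCharacter.
; Because the DoOnce precedes the cast, any other overlapping actor uses up the trigger.
; Spawns use hardcoded, evenly spaced world locations along Y, stretched on X, with collision handling set to always spawn.
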(event `self.Box.OnComponentBeginOverlap`
  (params (OverlappedComponent :type "PrimitiveComponent Object Reference") (OtherActor :type "Actor Object Reference") (OtherComp :type "PrimitiveComponent Object Reference") (OtherBodyIndex :type Integer) (bFromSweep :type Boolean) (SweepResult :type "HitResult Structure (by ref)"))
  (`/Engine/EditorBlueprintResources/StandardMacros.DoOnce` false
    (:`Completed`
      (`KismetSystemLibrary.PrintString` "Hello")
      (cast `/Game/ThirdPerson/Blueprints/BP_ThirdPersonCharacter` OtherActor)
      (`|SpawnActorFromClass` "/Game/LevelAssets/BP_RisingFlame.BP_RisingFlame_C" (`KismetMathLibrary.MakeTransform` (290.0 17740.0 -250.0) (struct) (3.25 1.0 1.0)) "AlwaysSpawn" "MultiplyWithRoot" null null)
      (`|SpawnActorFromClass` "/Game/LevelAssets/BP_RisingFlame.BP_RisingFlame_C" (`KismetMathLibrary.MakeTransform` (290.0 17870.0 -250.0) (struct) (3.25 1.0 1.0)) "AlwaysSpawn" "MultiplyWithRoot" null null)
      (`|SpawnActorFromClass` "/Game/LevelAssets/BP_RisingFlame.BP_RisingFlame_C" (`KismetMathLibrary.MakeTransform` (290.0 18000.0 -250.0) (struct) (3.25 1.0 1.0)) "AlwaysSpawn" "MultiplyWithRoot" null null)
      (`|SpawnActorFromClass` "/Game/LevelAssets/BP_RisingFlame.BP_RisingFlame_C" (`KismetMathLibrary.MakeTransform` (290.0 18130.0 -250.0) (struct) (3.25 1.0 1.0)) "AlwaysSpawn" "MultiplyWithRoot" null null)
      (`|SpawnActorFromClass` "/Game/LevelAssets/BP_RisingFlame.BP_RisingFlame_C" (`KismetMathLibrary.MakeTransform` (290.0 18260.0 -250.0) (struct) (3.25 1.0 1.0)) "AlwaysSpawn" "MultiplyWithRoot" null null)
      (`|SpawnActorFromClass` "/Game/LevelAssets/BP_RisingFlame.BP_RisingFlame_C" (`KismetMathLibrary.MakeTransform` (290.0 18390.0 -250.0) (struct) (3.25 1.0 1.0)) "AlwaysSpawn" "MultiplyWithRoot" null null)
      (`|SpawnActorFromClass` "/Game/LevelAssets/BP_RisingFlame.BP_RisingFlame_C" (`KismetMathLibrary.MakeTransform` (290.0 18520.0 -250.0) (struct) (3.25 1.0 1.0)) "AlwaysSpawn" "MultiplyWithRoot" null null)
      (`|SpawnActorFromClass` "/Game/LevelAssets/BP_RisingFlame.BP_RisingFlame_C" (`KismetMathLibrary.MakeTransform` (290.0 18650.0 -250.0) (struct) (3.25 1.0 1.0)) "AlwaysSpawn" "MultiplyWithRoot" null null))))

(fn `UserConstructionScript`)