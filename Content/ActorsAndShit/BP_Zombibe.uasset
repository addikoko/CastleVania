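; Zombie enemy that shuffles forward until AI perception picks up a target, then chases the player and dies from any damage.
; Perception updates start a looping timer that re-issues AI MoveTo on the player; forgetting the target halts the chase.
; A box overlap with the player's HurtBox deals damage, gated by a DoOnce that resets after a delay.
; Death plays Niagara, sound and animation before destroying the actor.
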(event `self.ReceiveTick`
  (params (DeltaSeconds :type "Float (single-precision)"))
  (if (not (`self.IS seeing player`))
    (`self.AddMovementInput` (`self.GetActorForwardVector`) 0.3)))

(event `self.Box.OnComponentBeginOverlap`
  (params (OverlappedComponent :type "PrimitiveComponent Object Reference") (OtherActor :type "Actor Object Reference") (OtherComp :type "PrimitiveComponent Object Reference") (OtherBodyIndex :type Integer) (bFromSweep :type Boolean) (SweepResult :type "HitResult Structure (by ref)"))
  (bind _asbp_third_person_character (cast `/Game/ThirdPerson/Blueprints/BP_ThirdPersonCharacter` OtherActor))
  (if (== OtherComp (`/Game/ThirdPerson/Blueprints/BP_ThirdPersonCharacter.HurtBox` _asbp_third_person_character))
    (set `self.Is Attacking` true)
    (`/Engine/EditorBlueprintResources/StandardMacros.DoOnce` false :!label _label
      (:`Completed`
        (`GameplayStatics.ApplyDamage` _asbp_third_person_character 10.0 null self)
        (`KismetSystemLibrary.Delay` 1.5)
        (goto _label :!via `Reset`)))))

(event `self.Test_AIPerception.OnTargetPerceptionUpdated`
  (params (Actor :type "Actor Object Reference") (Stimulus :type "AIStimulus Structure"))
  (set `self.IS seeing player` true)
  (`KismetSystemLibrary.K2_SetTimerDelegate` (delegate `Follow Player`) 1.0 true))

(event `self.ReceiveAnyDamage`
  (params (Damage :type "Float (single-precision)") (DamageType :type "DamageType Object Reference") (InstigatedBy :type "Controller Object Reference") (DamageCauser :type "Actor Object Reference"))
  (`self.EnemyDeath`))

(event `Follow Player`
  (if (`self.IS seeing player`)
    (`|AIMoveTo` self (`self.K2_GetActorLocation` (cast `/Game/ThirdPerson/Blueprints/BP_ThirdPersonCharacter` (`Controller.K2_GetPawn` (`GameplayStatics.GetPlayerController` 0)) :!pure true)) (`GameplayStatics.GetPlayerCharacter` 0))))

(event `EnemyDeath`
  (`AddComponent|NODE_AddNiagaraComponent-0`)
  (`GameplayStatics.PlaySound2D` "/Game/Music/deltarune_explosion_greenscreen.deltarune_explosion_greenscreen" 1.0 1.0 0.0 null null)
  (`SkeletalMeshComponent.PlayAnimation` (`self.Mesh`) "/Game/RENJASFOLDERGTO/3DModels/enemies/Zombie/Zombie_Death_Anim.Zombie_Death_Anim" false)
  (`KismetSystemLibrary.Delay` 1.5)
  (`self.K2_DestroyActor`))

(event `self.Test_AIPerception.OnTargetPerceptionForgotten`
  (params (Actor :type "Actor Object Reference"))
  (set `self.IS seeing player` false)
  (`|AIMoveTo` self (`self.K2_GetActorLocation` self) null))

(fn `UserConstructionScript`)