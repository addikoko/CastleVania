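; Crumbling stairs actor that sinks and destroys itself after the player character overlaps its R component.
; After SinkDelay, the Sink timeline lerps the actor down by SinkAmount from its current location.
; A two-second Delay on the timeline's Update leads to DestroyActor, so removal is timed from the sink's start.
; HasTriggered is set but never checked, as the branch condition is always true.
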(event `self.r.OnComponentBeginOverlap`
  (params (OverlappedComponent :type "PrimitiveComponent Object Reference") (OtherActor :type "Actor Object Reference") (OtherComp :type "PrimitiveComponent Object Reference") (OtherBodyIndex :type Integer) (bFromSweep :type Boolean) (SweepResult :type "HitResult Structure (by ref)"))
  (cast `/Game/ThirdPerson/Blueprints/BP_ThirdPersonCharacter` OtherActor)
  (if true
    (set `self.HasTriggered` true)
    (`KismetSystemLibrary.Delay` (`self.SinkDelay`))
    (set `self.StartLocation` (`self.K2_GetActorLocation`))
    (bind (_direction _alpha) (`Timeline|Sink`)
      (:`Update`
        (`self.K2_SetActorLocation` (`KismetMathLibrary.VLerp` (`self.StartLocation`) (+ (`self.StartLocation`) (`KismetMathLibrary.MakeVector` 0.0 0.0 (* (`self.SinkAmount`) -1.0))) _alpha))
        (`KismetSystemLibrary.Delay` 2.0)
        (`self.K2_DestroyActor`)))))

(fn `UserConstructionScript`)