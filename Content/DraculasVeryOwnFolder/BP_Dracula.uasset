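; BP_Dracula is a damageable Dracula actor, apparently an enemy, that leaves an all-clear orb when defeated.
; When BP_ThirdPersonCharacter overlaps its Box, it calls ApplyDamage on itself with the character as causer, but sets no base damage amount.
; AnyDamage subtracts incoming damage from Health; at zero or below it spawns BP_AllClearOrb at its location, then destroys itself after a short delay.
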(event `self.Box.OnComponentBeginOverlap`
  (params (OverlappedComponent :type "PrimitiveComponent Object Reference") (OtherActor :type "Actor Object Reference") (OtherComp :type "PrimitiveComponent Object Reference") (OtherBodyIndex :type Integer) (bFromSweep :type Boolean) (SweepResult :type "HitResult Structure (by ref)"))
  (bind _asbp_third_person_character (cast `/Game/ThirdPerson/Blueprints/BP_ThirdPersonCharacter` OtherActor))
  (`GameplayStatics.ApplyDamage` self 0.0 null _asbp_third_person_character))

(event `self.ReceiveAnyDamage`
  (params (Damage :type "Float (single-precision)") (DamageType :type "DamageType Object Reference") (InstigatedBy :type "Controller Object Reference") (DamageCauser :type "Actor Object Reference"))
  (bind _output_get (set `self.Health` (- (`self.Health`) (`self.Damage`))))
  (if (<= _output_get 0.0)
    (`|SpawnActorFromClass` "/Game/ActorsAndShit/BP_AllClearOrb.BP_AllClearOrb_C" (`KismetMathLibrary.MakeTransform` (`self.K2_GetActorLocation`)) "Undefined" "MultiplyWithRoot" null null)
    (`KismetSystemLibrary.Delay` 2.0)
    (`self.K2_DestroyActor`)))

(fn `UserConstructionScript`)